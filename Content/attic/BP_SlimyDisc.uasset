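; Slimy disc actor whose procedural mesh deforms to stick to surrounding geometry.
; Construction copies a hidden reference static mesh into the procedural mesh, and BeginPlay caches its original vertices.
; A fast looping timer traces from the mesh origin to each cached vertex on the Camera channel, pulling blocked vertices to hit points.
; The normal check compares a dot product to 45, so every blocking hit passes.
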(event `self.ReceiveBeginPlay`
  (bind _vertices (`KismetProceduralMeshLibrary.GetSectionFromProceduralMesh` (`self.ProceduralMesh`)))
  (set `self.VerticesArrayRef` _vertices)
  (`KismetSystemLibrary.K2_SetTimer` null "StickToEnvironment" 0.03 true true))

(fn `StickToEnvironment`
  (`KismetArrayLibrary.Array_Clear` (`self.VerticesArray`))
  (bind (_vertices _triangles _normals _uvs _tangents) (`KismetProceduralMeshLibrary.GetSectionFromProceduralMesh` (`self.ProceduralMesh`)))
  (for _array_element (`self.VerticesArrayRef`)
    (bind _outhit (`KismetSystemLibrary.LineTraceSingle` (`SceneComponent.K2_GetComponentLocation` (`self.ProceduralMesh`)) (`KismetMathLibrary.TransformLocation` (`self.GetTransform`) _array_element) "TraceTypeQuery2" false (`self.ActorsToIgnore`)))
    (if (`GameplayStatics.BreakHitResult` _outhit)
      (if (< (`KismetMathLibrary.Dot_VectorVector` (`.ImpactNormal` (`GameplayStatics.BreakHitResult` _outhit)) (`KismetMathLibrary.Vector_Up`)) 45.0)
        (`KismetArrayLibrary.Array_Add` (`self.VerticesArray`) (`KismetMathLibrary.InverseTransformLocation` (`self.GetTransform`) (`.Location` (`GameplayStatics.BreakHitResult` _outhit))))
        (else
          (`KismetArrayLibrary.Array_Add` (`self.VerticesArray`) _array_element :!label _label)))
      (else
        (goto _label))))
  (`ProceduralMeshComponent.UpdateMeshSection_LinearColor` :`self` (`self.ProceduralMesh`) :`Vertices` (`self.VerticesArray`) :`Normals` _normals :`UV0` _uvs :`Tangents` _tangents))

(fn `UserConstructionScript`
  (`KismetProceduralMeshLibrary.CopyProceduralMeshFromStaticMeshComponent` (`self.RefMesh`) 0 (`self.ProceduralMesh`))
  (`SceneComponent.SetVisibility` (`self.RefMesh`) false false))